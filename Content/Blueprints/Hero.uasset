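; Player pawn that walks between locations of a single prompt actor, collecting it to advance a task sequence.
; Movement axes feed a manual Tick move that applies consumed input as a swept local offset.
; Tick also tests distance to the prompt and toggles the take-task text on the ProcessCanvas widget.
; In range, TakePromt or OpenHistory opens history, creates the current task and moves the prompt to its next location.
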(event `InputAction|TakePromt`
  (params (Key :type "Key Structure"))
  (:`Pressed`
    (if (`self.isPromtVisible`)
      (`self.ProcessPromtGot`))))

(event `self.ReceiveBeginPlay`
  (bind _outactors (`GameplayStatics.GetAllActorsOfClass` "/Game/Blueprints/Promt.Promt_C"))
  (set `self.Promt` (`|GetArrayItem` _outactors))
  (bind _foundwidgets (`WidgetBlueprintLibrary.GetAllWidgetsOfClass` "/Game/UI/ProcessCanvas.ProcessCanvas_C"))
  (bind _output_get (set `self.ProcessCanvas` (`|GetArrayItem` _foundwidgets)))
  (`/Game/UI/ProcessCanvas.CreateTask` _output_get (`|GetArrayItem` (`self.AllPromtParams`)))
  (`/Game/UI/ProcessCanvas.CreateTask` (`self.ProcessCanvas`) (`|GetArrayItem` (`self.AllPromtParams`) 1)))

(event `InputAxis|MoveForward`
  (params (AxisValue :type "Float (single-precision)"))
  (`self.AddMovementInput` (`self.GetActorForwardVector`) (* AxisValue (`self.MaxSpeed`))))

(event `InputAxis|MoveRight`
  (params (AxisValue :type "Float (single-precision)"))
  (`self.AddMovementInput` (`self.GetActorRightVector`) (* AxisValue (`self.MaxSpeed`))))

(event `InputAction|OpenHistory`
  (params (Key :type "Key Structure"))
  (:`Pressed`
    (if (`self.isPromtVisible`)
      (`self.ProcessPromtGot`))))

(event `self.ReceiveTick`
  (params (DeltaSeconds :type "Float (single-precision)"))
  (`self.Move` DeltaSeconds)
  (`self.CheckPromtVisibility`)
  (`self.ProcessPromtVisibilityState`))

(fn `CheckPromtVisibility`
  (locals (DistToGetPromt :type "Float (double-precision)" :default 0.0))
  (set `self.isPromtVisible` (<= (`KismetMathLibrary.Vector_Distance` (`SceneComponent.K2_GetComponentLocation` (`self.RootComponent`)) (`SceneComponent.K2_GetComponentLocation` (`Actor.RootComponent` (`self.Promt`)))) (`local.DistToGetPromt`)))
  (return))

(fn `Move`
  (params (B :type "Float (double-precision)"))
  (bind _returnvalue (`self.ConsumeMovementInputVector`))
  (`self.K2_AddActorLocalOffset` (* _returnvalue B) true))

(fn `ProcessPromtGot`
  (locals (CurParams :type "/Game/Blueprints/StructPromtParams Structure"))
  (bind _processcanvas (`self.ProcessCanvas`))
  (bind (_output_istask _output_begintext _output_taskparams _output_nextlocation) (break `/Game/Blueprints/StructPromtParams` (`|GetArrayItem` (`self.AllPromtParams`) (`self.CurrentPromtId`))))
  (set `local.CurParams` (`|GetArrayItem` (`self.AllPromtParams`) (`self.CurrentPromtId`)))
  (`/Game/UI/ProcessCanvas.OpenHistory` _processcanvas)
  (`/Game/UI/ProcessCanvas.CreateTask` _processcanvas (`local.CurParams`))
  (`self.K2_SetActorLocation` (`self.Promt`) _output_nextlocation false false)
  (`/Engine/EditorBlueprintResources/StandardMacros.IncrementInt` (`self.CurrentPromtId`)))

(fn `ProcessPromtInvisible`)

(fn `ProcessPromtVisibilityState`
  (if (`self.isPromtVisible`)
    (`/Game/UI/ProcessCanvas.ChangeVisibilityOfTakeTaskText` (`self.ProcessCanvas`) "Visible")
    (else
      (`/Game/UI/ProcessCanvas.ChangeVisibilityOfTakeTaskText` (`self.ProcessCanvas`) "Hidden"))))

(fn `ProcessPromtVisible`)

(fn `UserConstructionScript`)